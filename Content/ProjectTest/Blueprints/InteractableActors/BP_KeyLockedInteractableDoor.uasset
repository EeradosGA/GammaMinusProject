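; BP_KeyLockedInteractableDoor is an interactable door that only responds when the player carries its required key.
; Interact searches the pawn's interactable-actor inventory for the referenced key actor and calls the parent interaction only if it is found.
; Otherwise it plays the disappear animation on a key-needed popup widget, which is created and added to the player screen at BeginPlay.
; An unset key reference keeps the door locked.
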(event `self.ReceiveBeginPlay`
  (`parent.ReceiveBeginPlay`)
  (bind _returnvalue (`|CreateWidget` "/Game/ProjectTest/Blueprints/UI/WBP_PopUpKeyNeeded.WBP_PopUpKeyNeeded_C"))
  (bind _output_get (set `self.WBP_PopUpKeyNeededRef` _returnvalue))
  (`UserWidget.AddToPlayerScreen` _output_get 0))

(event `InteractableInterface.Interact`
  (bind _wbp_popupkeyneededref (`self.WBP_PopUpKeyNeededRef`))
  (bind _asmy_pawn (cast `MyPawn` (`Controller.K2_GetPawn` (`GameplayStatics.GetPlayerController` 0))))
  (bind _hasfounditemininventory (`self.FindKeyNeededInPlayerInventory` _asmy_pawn))
  (if _hasfounditemininventory
    (`parent.Interact`)
    (else
      (`UserWidget.PlayAnimation` _wbp_popupkeyneededref (`/Game/ProjectTest/Blueprints/UI/WBP_PopUpKeyNeeded.DisappearAnim` _wbp_popupkeyneededref) 0.0 1 "Forward" 1.0 false))))

(fn `FindKeyNeededInPlayerInventory`
  (params (_PlayerToCheck :type "MyPawn Object Reference"))
  (returns (HasFoundItemInInventory :type Boolean))
  (`/Engine/EditorBlueprintResources/StandardMacros.IsValid` (`self.BP_KeyNeeded`)
    (:`Is Valid`
      (return (!= (`KismetArrayLibrary.Array_Find` (`MyPawn.GetInventoryActorInteractable` _PlayerToCheck) (`self.BP_KeyNeeded`)) -1)))
    (:`Is Not Valid`
      (return false))))

(fn `UserConstructionScript`
  (`parent.UserConstructionScript`))