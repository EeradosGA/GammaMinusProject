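; BP_KeyInteractable is an interactable key that the player picks up into their inventory.
; On Interact, it runs the parent logic, adds itself to the MyPawn inventory, then destroys its Sphere and StaticMesh components, leaving the actor alive.
; While flagged as being interacted with, Tick snaps the actor to the controlled pawn's location every frame.
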(event `self.ReceiveBeginPlay`
  (`parent.ReceiveBeginPlay`))

(event `self.ReceiveTick`
  (params (DeltaSeconds :type "Float (single-precision)"))
  (`parent.ReceiveTick` DeltaSeconds)
  (if (`self.GetIsBeingInteractWith`)
    (`self.K2_SetActorLocation` (`self.K2_GetActorLocation` (`Controller.K2_GetPawn` (`GameplayStatics.GetPlayerController` 0))))))

(event `InteractableInterface.Interact`
  (`parent.Interact`)
  (bind _asmy_pawn (cast `MyPawn` (`Controller.K2_GetPawn` (`GameplayStatics.GetPlayerController` 0))))
  (`MyPawn.AddActorInteractableToInventory` _asmy_pawn self)
  (`ActorComponent.K2_DestroyComponent` (`self.Sphere`))
  (`ActorComponent.K2_DestroyComponent` (`self.StaticMesh`)))

(fn `UserConstructionScript`)